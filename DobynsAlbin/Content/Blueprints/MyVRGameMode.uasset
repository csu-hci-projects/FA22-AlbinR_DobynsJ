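; MyVRGameMode is a game mode that respawns the player's VR pawn after it is destroyed.
; On BeginPlay it binds to the destroyed event of player 0's MyVRPawn.
; When that pawn is destroyed, it waits briefly, spawns a new MyVRPawn at RespawnTransform, has the player controller possess it, then calls Respawn to bind the event again.
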(event Custom|OnDestroyed_Event_0
  (params (DestroyedActor :type Actor%20Object%20Reference))
  (Utilities|FlowControl|Delay 1.0)
  (bind _returnvalue (Game|SpawnActorfromClass "/Game/Blueprints/MyVRPawn.MyVRPawn_C" (Variables|Default|GetRespawn%20%20Transform) "Undefined" 0 0)) ; respawn MyVRPawn
  (Pawn|Possess (Game|GetPlayerController 0) _returnvalue)
  (CallFunction|Respawn))

(event Custom|Respawn
  (bind _asmy_vrpawn (Utilities|Casting|CastToMyVRPawn (Game|Player|GetPlayerPawn 0))) ; cast to MyVRPawn
  (Game|AssignOnDestroyed _asmy_vrpawn (delegate Custom|OnDestroyed_Event_0)))

(event EventBeginPlay
  (bind _asmy_vrpawn (Utilities|Casting|CastToMyVRPawn (Game|Player|GetPlayerPawn 0))) ; cast to MyVRPawn
  (Game|AssignOnDestroyed _asmy_vrpawn (delegate Custom|OnDestroyed_Event_0)))

(event EventTick
  (params (DeltaSeconds :type Float%20%28single-precision%29))
  (|CallParentFunction DeltaSeconds) ; This node is disabled and will not be called.\nDrag off pins to build functionality.
)

(fn ConstructionScript
  (|CallParentFunction))